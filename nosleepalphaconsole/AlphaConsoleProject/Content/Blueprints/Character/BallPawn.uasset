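; Physics-driven ball pawn that moves by force on its BallCase and carries a separately rotated Camera.
; Each tick, movement input X/Y becomes a force rotated to the ball's heading, while Z sets its yaw spin.
; The Camera receives roll and pitch computed from velocity and circumference to mimic rolling, plus local rotation from SecondInput.
; The intended stopping-damping boost is unwired, so linear damping stays low.
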(event Custom|Consume%20Second%20Input
  (params (NewParam :type Vector))
  ;[0 0.9572 1] Take in the Second Input vector
  (Variables|Default|SetSecondInput NewParam))

(event EventBeginPlay
  ;[0.4709 0 1] Calculate scale for rotation by radius and velocity
  (Variables|Default|SetCirumference (* (Math|Float|MultiplybyPi 5e+01) 2.0)))

(event EventTick
  (params (DeltaSeconds :type Float%20%28single-precision%29))
  ;[0.528 1 0] What to do with the ball every tick
  (bind _output_get (Variables|Default|SetDeltaTime DeltaSeconds))
  (bind _zinput (CallFunction|MoveBall))
  (bind _deltarotation (CallFunction|CalcMovementRotation _output_get 1))
  (CallFunction|ApplyMovementRotation _deltarotation)
  (CallFunction|ApplyCameraRotation)
  ;;[1 0 0.07801] Spin the ball
  (Class|PrimitiveComponent|SetPhysicsAngularVelocity (Variables|Default|GetBallCase) (Math|Vector|MakeVector 0.0 0.0 (* _zinput (Variables|Default|GetCamRotSpeed))) false "None"))

(fn ConstructionScript)

(fn MoveBall
  (bind _returnvalue (Class|Pawn|ConsumeMovementInputVector))
  ;[0.5 0 1] Augmented Damping to stop
  (if (< (Math|Vector|VectorLengthSquared _returnvalue) 0.01)
    _
    (else
      _))
  (Class|PrimitiveComponent|SetLinearDamping (Variables|Default|GetBallCase) 0.001)
  ;[1 0 0.05385] Account for Ball Rotation
  (bind _angle (CallFunction|AngleBetween "1.000000, 0, 0" (Math|Vector|GetForwardVector (Variables|Default|GetBallCase))))
  (Development|PrintText (Utilities|Text|ToText(Float) _angle "HalfToEven"))
  (Physics|AddForce (Variables|Default|GetBallCase) (Math|Vector|RotateVectorAroundAxis (* (Math|Vector|MakeVector (.X (Math|Vector|BreakVector _returnvalue)) (.Y (Math|Vector|BreakVector _returnvalue)) 0.0) (Variables|Default|GetForceAdjustment)) _angle "0, 0,1.000000") "None" false)
  (return (.Z (Math|Vector|BreakVector _returnvalue))))

(fn CalcMovementRotation
  (params (deltaTime :type Float%20%28single-precision%29) (Modifier :type Integer))
  (bind _ballcase (Variables|Default|GetBallCase))
  (bind _returnvalue (Transformation|GetComponentVelocity _ballcase))
  (return (Math|Vector|RotatorfromAxisandAngle (Math|Vector|CrossProduct (Math|Vector|GetUpVector _ballcase) _returnvalue) (* (/ (Math|Vector|VectorLength _returnvalue) (Variables|Default|GetCirumference)) deltaTime 3.6e+02))))

(fn ApplyMovementRotation
  (params (InRot :type Rotator))
  (bind (_roll _pitch) (Math|Rotator|BreakRotator InRot))
  (Transformation|AddWorldRotation (Variables|Default|GetCamera) (Math|Rotator|MakeRotator _roll _pitch 0.0) false false))

(fn AngleBetween
  (params (V1 :type Vector) (V2 :type Vector))
  (bind _returnvalue (Math|Vector|Normalize V1))
  (bind _returnvalue_2 (Math|Vector|Normalize V2))
  (bind _returnvalue_3 (Math|Vector|DotProduct _returnvalue _returnvalue_2))
  (bind _returnvalue_4 (Class|KismetMathLibrary|DegAcos _returnvalue_3))
  ;[1 1 1] Make the angle negative in the upper half according to positive world rotation
  (if (< (- (.Y (Math|Vector|BreakVector V1)) (.Y (Math|Vector|BreakVector V2))) 0.0)
    (return _returnvalue_4)
    (else
      (bind _result (Math|Float|NegateFloat _returnvalue_4)
        (:%20%20
          (return _result))))))

(fn ApplyCameraRotation
  (bind _secondinput (Variables|Default|GetSecondInput))
  (bind _camrotspeed (Variables|Default|GetCamRotSpeed))
  (bind _deltatime (Variables|Default|GetDeltaTime))
  (bind (_x _y _z) (Math|Vector|BreakVector _secondinput))
  (Transformation|AddLocalRotation (Variables|Default|GetCamera) (Math|Rotator|MakeRotator (* _x _deltatime _camrotspeed) (* _y _camrotspeed _deltatime) (* _z _camrotspeed _deltatime)) false false)
  (return))