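; Player controller that splits control of a BallPawn between local players by controller ID parity and handles pause menu input.
; Even IDs move their own pawn through movement input, while odd IDs view player 0's pawn and feed stick input into NetInput, which Tick passes to ConsumeSecondInput.
; X freezes the ball while held; UI actions fire dispatchers and open or close PauseMenuWidget, and Q toggles IsPlaying for debugging.
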(event EventBeginPlay
  ;[1 0.7575 0] Determine which state this should be in
  (bind _returnvalue (CallFunction|DetermineState))
  (bind _output_get (Variables|Default|SetEvenID _returnvalue))
  (if _output_get
    ;[1 0 0] Set Up Ball Controller
    (bind _asball_pawn (Utilities|Casting|CastToBallPawn (Game|Player|GetPlayerPawn (Variables|Default|GetMyID)))
      (:then
        (Variables|Default|SetPlayerBall _asball_pawn))
      (:CastFailed
        ;[0 1 0.08889] Set Up Camera Controller
        (Development|PrintText "Player Ball could not be found" true true "(R=1.000000,G=0.000000,B=0.000000,A=1.000000)" :!label _label)))
    (else
      (Game|Player|SetViewTargetwithBlend (Game|Player|GetPlayerPawn 0) 0.0 "VTBlend_Linear" 0.0 false)
      (Variables|Default|SetPlayerCam (Actor|GetComponentbyClass (Game|Player|GetPlayerPawn 0) "/Script/Engine.CameraComponent"))
      (bind _asball_pawn_2 (Utilities|Casting|CastToBallPawn (Game|Player|GetPlayerPawn 0))
        (:then
          (Variables|Default|SetPlayerBall _asball_pawn_2))
        (:CastFailed
          (goto _label))))))

(event EventTick
  (params (DeltaSeconds :type Float%20%28single-precision%29))
  ;[0 1 0.08889] Potentially update pawn with Camera Net Input
  (if (not (Variables|Default|GetEvenID))
    (Default|ConsumeSecondInput (Variables|Default|GetPlayerBall) (Variables|Default|GetNetInput))
    (Variables|Default|SetNetInput "0, 0, 0")))

(event Input|ActionEvents|InputActionXButton
  (params (Key :type Key%20Structure))
  (bind _playerball (Variables|Default|GetPlayerBall))
  (:Pressed
    (Default|FreezeBall _playerball))
  (:Released
    (Default|UnFreezeBall _playerball)))

(event Input|ActionEvents|InputActionUI_Select
  (params (Key :type Key%20Structure))
  ;[1 1 1] UI Pause Menu Functionality
  (:Pressed
    (Default|CallSelectDispatcher Key)))

(event Input|ActionEvents|InputActionUI_Pause
  (params (Key :type Key%20Structure))
  ;[1 1 1] UI Pause Menu Functionality
  (:Pressed
    (Default|CallPauseDispatcher Key)
    (if (Variables|Default|GetisScreenShown)
      (bind _foundwidgets (Widget|GetAllWidgetsOfClass "/Game/Blueprints/MainGameBlueprints/PauseMenu/PauseMenuWidget.PauseMenuWidget_C" true))
      (for _array_element _foundwidgets
        (Default|UnPauseGame _array_element))
      (else
        (bind _returnvalue (UserInterface|CreateWidget "/Game/Blueprints/MainGameBlueprints/PauseMenu/PauseMenuWidget.PauseMenuWidget_C"))
        (UserInterface|Viewport|AddtoViewport _returnvalue 0)
        (bind _output_get (Variables|/Game/Blueprints/MainGameBlueprints/PauseMenu/PauseMenuWidget.PauseMenuWidget_C|SetpauseID _returnvalue (Variables|Default|GetEvenID)))
        (if _output_get
          (Input|SetInputModeGameandUI (Game|GetPlayerController 0) _returnvalue "DoNotLock" true)
          (Variables|Default|SetbShowMouseCursor true)
          (Variables|Default|SetisScreenShown true)
          (Game|SetGamePaused true)
          (else
            (Input|SetInputModeGameandUI (Game|GetPlayerController 1) 0 "DoNotLock" true)
            (Variables|Default|SetbShowMouseCursor true)
            (Variables|Default|SetisScreenShown true)
            (Game|SetGamePaused true)))))))

(event Input|ActionEvents|InputActionUI_Down
  (params (Key :type Key%20Structure))
  ;[1 1 1] UI Pause Menu Functionality
  (:Pressed
    (Default|CallDPadDownDispatcher Key)))

(event Input|ActionEvents|InputActionUI_Up
  (params (Key :type Key%20Structure))
  ;[1 1 1] UI Pause Menu Functionality
  (:Pressed
    (Default|CallDPadUpDispatcher Key)))

(event Input|ActionEvents|InputActionBack
  (params (Key :type Key%20Structure))
  ;[1 1 1] UI Pause Menu Functionality
  (:Pressed
    (Default|CallUIBackDispatcher Key)
    (if (Variables|Default|GetisScreenShown)
      (bind _foundwidgets (Widget|GetAllWidgetsOfClass "/Game/Blueprints/MainGameBlueprints/PauseMenu/PauseMenuWidget.PauseMenuWidget_C" true))
      (for _array_element _foundwidgets
        (if (Variables|/Game/Blueprints/MainGameBlueprints/PauseMenu/PauseMenuWidget.PauseMenuWidget_C|GetisOptionScreenOpen _array_element)
          (Default|CloseMenu _array_element)
          (else
            (Default|UnPauseGame _array_element)))))))

(event Input|AxisEvents|InputAxisRStickX
  (params (AxisValue :type Float%20%28single-precision%29))
  (bind _playerball (Variables|Default|GetPlayerBall))
  ;[1 0.9621 0] Calculate RStickX Action
  (if (Variables|Default|GetEvenID)
    (Pawn|Input|AddMovementInput _playerball (Transformation|GetActorUpVector _playerball) AxisValue false)
    (else
      (Variables|Default|SetNetInput (+ (Math|Vector|MakeVector 0.0 0.0 AxisValue) (Variables|Default|GetNetInput))))))

(event Input|AxisEvents|InputAxisRStickY
  (params (AxisValue :type Float%20%28single-precision%29))
  ;[0.0638 1 0] RStickY action
  (if (not (Variables|Default|GetEvenID))
    (Variables|Default|SetNetInput (+ (Math|Vector|MakeVector 0.0 AxisValue 0.0) (Variables|Default|GetNetInput)))))

(event Input|AxisEvents|InputAxisLStickX
  (params (AxisValue :type Float%20%28single-precision%29))
  (bind _playerball (Variables|Default|GetPlayerBall))
  ;[1 0.7635 0] Calculate LStickX action
  (if (Variables|Default|GetEvenID)
    (Pawn|Input|AddMovementInput _playerball (Transformation|GetActorRightVector _playerball) AxisValue false)
    (else
      (Variables|Default|SetNetInput (+ (Math|Vector|MakeVector AxisValue 0.0 0.0) (Variables|Default|GetNetInput))))))

(event Input|AxisEvents|InputAxisLStickY
  (params (AxisValue :type Float%20%28single-precision%29))
  (bind _playerball (Variables|Default|GetPlayerBall))
  ;[1 0.7635 0] Calculate LStickY action
  (if (Variables|Default|GetEvenID)
    (Pawn|Input|AddMovementInput _playerball (Transformation|GetActorForwardVector _playerball) AxisValue false)))

(event Input|KeyboardEvents|Q
  (params (Key :type Key%20Structure))
  ;[1 1 1] debug command
  (:Pressed
    (bind _asmain_game_mode (Utilities|Casting|CastToMainGameMode (Game|GetGameMode)))
    (Variables|/Game/Blueprints/MainGameBlueprints/MainGameMode.MainGameMode_C|SetisPlaying _asmain_game_mode (not (Variables|/Game/Blueprints/MainGameBlueprints/MainGameMode.MainGameMode_C|GetisPlaying _asmain_game_mode)))))

(fn ConstructionScript)

(fn DetermineState
  (bind _returnvalue (Class|GameplayStatics|GetPlayerControllerID self))
  (Development|PrintText (Utilities|Text|ToText(Integer) _returnvalue))
  (Variables|Default|SetMyID _returnvalue)
  (return (== (Math|Integer|%(Integer) _returnvalue 2) 0)))