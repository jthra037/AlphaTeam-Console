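; CameraController sets the view to the player pawn and relays gamepad stick input to the BallPawn.
; BeginPlay caches the pawn's camera and ball references, printing a red error if the BallPawn cast fails.
; Axis events accumulate left stick X/Y and right stick X into one vector, which Tick passes to ConsumeSecondInput and then clears.
; Both accumulation and forwarding run only while MainGameMode reports IsPlaying.
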(event EventBeginPlay
  (Game|Player|SetViewTargetwithBlend (Game|Player|GetPlayerPawn 0) 0.0 "VTBlend_Linear" 0.0 false)
  (Variables|Default|SetPlayerCam (Actor|GetComponentbyClass (Game|Player|GetPlayerPawn 0) "/Script/Engine.CameraComponent"))
  (bind _asball_pawn (Utilities|Casting|CastToBallPawn (Game|Player|GetPlayerPawn 0))
    (:then
      (Variables|Default|SetPlayerBall _asball_pawn))
    (:CastFailed
      (Development|PrintText "Player Ball could not be found" true true "(R=1.000000,G=0.000000,B=0.000000,A=1.000000)"))))

(event EventTick
  (params (DeltaSeconds :type Float%20%28single-precision%29))
  (bind _asmain_game_mode (Utilities|Casting|CastToMainGameMode (Game|GetGameMode)))
  (if (Variables|/Game/Blueprints/MainGameBlueprints/MainGameMode.MainGameMode_C|GetisPlaying _asmain_game_mode)
    (Default|ConsumeSecondInput (Variables|Default|GetPlayerBall) (Variables|Default|GetNetInput))
    (Variables|Default|SetNetInput "0, 0, 0")))

(event Input|AxisEvents|InputAxisRStickX
  (params (AxisValue :type Float%20%28single-precision%29))
  (bind _asmain_game_mode (Utilities|Casting|CastToMainGameMode (Game|GetGameMode)))
  (if (Variables|/Game/Blueprints/MainGameBlueprints/MainGameMode.MainGameMode_C|GetisPlaying _asmain_game_mode)
    (Variables|Default|SetNetInput (+ (Math|Vector|MakeVector 0.0 0.0 AxisValue) (Variables|Default|GetNetInput)))))

(event Input|AxisEvents|InputAxisLStickX
  (params (AxisValue :type Float%20%28single-precision%29))
  (bind _asmain_game_mode (Utilities|Casting|CastToMainGameMode (Game|GetGameMode)))
  (if (Variables|/Game/Blueprints/MainGameBlueprints/MainGameMode.MainGameMode_C|GetisPlaying _asmain_game_mode)
    (Variables|Default|SetNetInput (+ (Math|Vector|MakeVector AxisValue 0.0 0.0) (Variables|Default|GetNetInput)))))

(event Input|AxisEvents|InputAxisLStickY
  (params (AxisValue :type Float%20%28single-precision%29))
  (bind _asmain_game_mode (Utilities|Casting|CastToMainGameMode (Game|GetGameMode)))
  (if (Variables|/Game/Blueprints/MainGameBlueprints/MainGameMode.MainGameMode_C|GetisPlaying _asmain_game_mode)
    (Variables|Default|SetNetInput (+ (Math|Vector|MakeVector 0.0 AxisValue 0.0) (Variables|Default|GetNetInput)))))

(fn ConstructionScript)