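; GateButtonActor is a button actor in the ShootTest folder that triggers gate destruction when hit by a projectile.
; On overlap, it checks the other actor's tags for "Projectile" and calls CallDestroyGate, whose body is not in this graph.
; An unconnected chain would damage the Destructible of every GateActor and set IsGateDestroyed to prevent repeats, but it never runs.
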(event EventBeginPlay)

(event Collision|EventActorBeginOverlap
  (params (OtherActor :type Actor%20Object%20Reference))
  (for _array_element (Variables|/Script/Engine.Actor|GetTags OtherActor)
    (if (Utilities|Name|Equal(Name) _array_element "Projectile")
      (Default|CallDestroyGate))))

(event EventTick
  (params (DeltaSeconds :type Float%20%28single-precision%29)))

(fn ConstructionScript)