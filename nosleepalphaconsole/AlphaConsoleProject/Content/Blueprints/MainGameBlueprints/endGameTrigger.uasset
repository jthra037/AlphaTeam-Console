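; End-of-level trigger that stops play when the player pawn overlaps it and swaps the HUD for the end-game widget.
; AddScore rebuilds the level's saved leaderboard, inserting the final score in ascending order as "Player 1" with the date.
; AchievementCheck, called from the HUD removal loop, saves a low-score achievement.
; Both use per-level save slots named from the level name, with DoOnce guarding against repeat runs.
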(event EventBeginPlay)

(event Collision|EventActorBeginOverlap
  (params (OtherActor :type Actor%20Object%20Reference))
  (if (== OtherActor (Game|Player|GetPlayerPawn 0))
    (bind _asmain_game_mode (Utilities|Casting|CastToMainGameMode (Game|GetGameMode)))
    (Variables|/Game/Blueprints/MainGameBlueprints/MainGameMode.MainGameMode_C|SetisPlaying _asmain_game_mode false)
    (CallFunction|AddScore "None" (Variables|/Game/Blueprints/MainGameBlueprints/MainGameMode.MainGameMode_C|GetfinalScore _asmain_game_mode))
    (bind _returnvalue (UserInterface|CreateWidget "/Game/Blueprints/MainGameBlueprints/endGameWidget.endGameWidget_C"))
    (UserInterface|Viewport|AddtoViewport _returnvalue 0)
    (bind _foundwidgets (Widget|GetAllWidgetsOfClass "/Game/Blueprints/MainGameBlueprints/HUDWidget.HUDWidget_C" true))
    (for _array_element _foundwidgets
      (Widget|RemovefromParent _array_element)
      (CallFunction|AchievementCheck))))

(event EventTick
  (params (DeltaSeconds :type Float%20%28single-precision%29)))

(fn ConstructionScript)

(fn AddScore
  (params (MapName :type Name) (Score :type Integer))
  (bind _temp (Variables|Default|Gettemp))
  (Variables|Default|SetmScore Score)
  (Utilities|FlowControl|DoOnce false
    (:Completed
      (bind _returnvalue (Game|GetCurrentLevelName true))
      (bind _returnvalue_2 (SaveGame|LoadGamefromSlot (Utilities|String|Append _returnvalue "-Leaderboards")))
      (bind _asscore_save (Utilities|Casting|CastToscoreSave _returnvalue_2)
        (:then
          (for _array_element (Variables|/Game/Blueprints/LeaderBoards/scoreSave.scoreSave_C|GetPlayerScores _asscore_save)
            (Utilities|FlowControl|Sequence
              (:then_0
                (if (>= (.score (Utilities|Struct|BreakplayerScore _array_element)) (Variables|Default|GetmScore))
                  (Utilities|FlowControl|DoOnce false
                    (:Completed
                      (if (<= (Utilities|Array|Length (Variables|/Game/Blueprints/LeaderBoards/scoreSave.scoreSave_C|GetPlayerScores _asscore_save)) 1)
                        _
                        (else
                          (Utilities|Array|RemoveIndex (Variables|/Game/Blueprints/LeaderBoards/scoreSave.scoreSave_C|GetPlayerScores _asscore_save) (- (Utilities|Array|Length (Variables|/Game/Blueprints/LeaderBoards/scoreSave.scoreSave_C|GetPlayerScores _asscore_save)) 10))))
                      (Utilities|Array|Add _temp (Utilities|Struct|MakeplayerScore "Player 1" (Variables|Default|GetmScore) (Class|KismetMathLibrary|GetDate)))))))
              (:then_1
                (Utilities|Array|Add _temp _array_element))))
          (Utilities|FlowControl|Sequence
            (:then_0
              (Utilities|FlowControl|DoOnce false :!label _label
                (:Completed
                  (if (<= (Utilities|Array|Length (Variables|/Game/Blueprints/LeaderBoards/scoreSave.scoreSave_C|GetPlayerScores _asscore_save)) 1)
                    _
                    (else
                      (Utilities|Array|RemoveIndex (Variables|/Game/Blueprints/LeaderBoards/scoreSave.scoreSave_C|GetPlayerScores _asscore_save) (- (Utilities|Array|Length (Variables|/Game/Blueprints/LeaderBoards/scoreSave.scoreSave_C|GetPlayerScores _asscore_save)) 10))))
                  (Utilities|Array|Add _temp (Utilities|Struct|MakeplayerScore "Player 1" (Variables|Default|GetmScore) (Class|KismetMathLibrary|GetDate))))))
            (:then_1
              (bind _returnvalue_3 (SaveGame|CreateSaveGameObject "/Game/Blueprints/LeaderBoards/scoreSave.scoreSave_C" :!label _label_2))
              (Variables|/Game/Blueprints/LeaderBoards/scoreSave.scoreSave_C|SetPlayerScores _returnvalue_3 _temp)
              (bind _returnvalue_4 (Game|GetCurrentLevelName true))
              (SaveGame|SaveGametoSlot _returnvalue_3 (Utilities|String|Append _returnvalue_4 "-Leaderboards")))))
        (:CastFailed
          (Utilities|FlowControl|Sequence
            (:then_0
              (goto _label))
            (:then_1
              (goto _label_2))))))))

(fn AchievementCheck
  (Utilities|FlowControl|DoOnce false
    (:Completed
      (bind _returnvalue (Game|GetCurrentLevelName true))
      (bind _returnvalue_2 (SaveGame|LoadGamefromSlot (Utilities|String|Append _returnvalue "-Achievements")))
      (Utilities|Casting|CastToAchievementsSave _returnvalue_2
        (:then
          (bind _asmain_game_mode (Utilities|Casting|CastToMainGameMode (Game|GetGameMode)))
          (if (<= (Variables|/Game/Blueprints/MainGameBlueprints/MainGameMode.MainGameMode_C|GetfinalScore _asmain_game_mode) 5)
            (bind _returnvalue_3 (SaveGame|CreateSaveGameObject "/Game/Blueprints/Achievements/AchievementsSave.AchievementsSave_C"))
            (Variables|/Game/Blueprints/Achievements/AchievementsSave.AchievementsSave_C|SetAchievements _returnvalue_3 (Utilities|Struct|MakeAchievement (<= (Variables|/Game/Blueprints/MainGameBlueprints/MainGameMode.MainGameMode_C|GetfinalScore _asmain_game_mode) 5)))
            (SaveGame|SaveGametoSlot _returnvalue_3 (Utilities|String|Append _returnvalue "-Achievements"))))
        (:CastFailed
          (bind _returnvalue_4 (SaveGame|CreateSaveGameObject "/Game/Blueprints/Achievements/AchievementsSave.AchievementsSave_C"))
          (bind _asmain_game_mode_2 (Utilities|Casting|CastToMainGameMode (Game|GetGameMode)))
          (Variables|/Game/Blueprints/Achievements/AchievementsSave.AchievementsSave_C|SetAchievements _returnvalue_4 (Utilities|Struct|MakeAchievement (<= (Variables|/Game/Blueprints/MainGameBlueprints/MainGameMode.MainGameMode_C|GetfinalScore _asmain_game_mode_2) 5)))
          (SaveGame|SaveGametoSlot _returnvalue_4 (Utilities|String|Append _returnvalue "-Achievements")))))))